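; Game mode for Luthenium that sets up the monster and the tutorial at BeginPlay.
; It spawns BP_Monseter at a local-variable location and caches its BP_AI_MonsterController, leaving MonsterSpawnLocation unused.
; After short delays, SpawnMonsterTargets gathers existing BP_Monster_Target actors rather than spawning any, hands them to the controller and starts movement from the first target.
; BPM_Tutorial then spawns at the world origin.
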(event `self.ReceiveBeginPlay`
  (`KismetSystemLibrary.Delay` 1.0)
  (`self.Spawn Moster`)
  (`KismetSystemLibrary.Delay` 1.0)
  (`self.Spawn Monster Targets`)
  (`|SpawnActorFromClass` "/Game/Blueprints/GameMode/BPM_Tutorial.BPM_Tutorial_C" (`KismetMathLibrary.MakeTransform` (0.0 0.0 0.0)) "AlwaysSpawn" "OverrideRootScale" null null))

(fn `Spawn Monster Targets`
  (bind _monster_ai_controller (`self.Monster AI controller`))
  (bind _outactors (`GameplayStatics.GetAllActorsOfClass` "/Game/Blueprints/GameMode/BP_Monster_Target.BP_Monster_Target_C"))
  (bind _output_get (set `self.Monster Targets` _outactors))
  (`/Engine/EditorBlueprintResources/StandardMacros.IsValid` _monster_ai_controller
    (:`Is Valid`
      (set `MonsterAIController.Targets` _output_get _monster_ai_controller)
      (`MonsterAIController.StartMovingToNextTargetLocation` _monster_ai_controller 0 true)
      (`KismetSystemLibrary.PrintString` "Hello"))))

(fn `Spawn Moster`
  (locals (NewLocalVar_0 :type "Vector Structure" :default (-534614.6875 73401.34375 86678.484375)))
  (bind _returnvalue (`|SpawnActorFromClass` "/Game/Blueprints/Monster/BP_Monseter.BP_Monseter_C" (`KismetMathLibrary.MakeTransform` (`local.NewLocalVar_0`)) "AlwaysSpawn" "OverrideRootScale" null null))
  (bind _output_get (set `self.Monster` _returnvalue))
  (bind _returnvalue_2 (`AIBlueprintHelperLibrary.GetAIController` _output_get))
  (`/Engine/EditorBlueprintResources/StandardMacros.IsValid` _returnvalue_2
    (:`Is Valid`
      (bind _asbp_ai_monster_controller (cast `/Game/Blueprints/Monster/BP_AI_MonsterController` _returnvalue_2))
      (set `self.Monster AI controller` _asbp_ai_monster_controller))))

(fn `UserConstructionScript`)