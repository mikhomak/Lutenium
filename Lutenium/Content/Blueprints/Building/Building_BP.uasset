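; Procedural building actor that assembles a block-based building from instanced meshes in its Construction Script, with no active runtime logic.
; It loops over floors, segments and width, intended to fill only the outer shell and top floor.
; Each block becomes foundation or porch at ground level, normal or balcony above.
; Upper-floor blocks also get a dryer or air conditioner at a random window, offset and rotated by facade direction.
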(fn `Init Block`
  (params (Floor :type Integer) (Segment :type Integer) (`Segment WIdth` :type Integer))
  (returns (`Balcony?` :type Boolean) (Position :type "Vector Structure"))
  (bind _position (`self.Caclulate Block Position` Floor Segment `Segment WIdth`))
  (bind _balcony_ (`self.Should it be balcony?` Floor Segment `Segment WIdth`))
  (`self.Calculate current direction` Segment `Segment WIdth`
    (:`Finish`
      (if (!= Floor 0)
        (if _balcony_
          ;[1 1 1] Balcony Block
          (`InstancedStaticMeshComponent.AddInstance` (`self.Balcony Block`) (`KismetMathLibrary.MakeTransform` _position (`self.Current Rotation`)))
          (else
            ;[1 1 1] Normal Block
            (`InstancedStaticMeshComponent.AddInstance` (`self.Block`) (`KismetMathLibrary.MakeTransform` _position))))
        (else
          ;[1 1 1] Foundation blocks
          (if (`self.Should fundation be porch?` Segment)
            (`InstancedStaticMeshComponent.AddInstance` (`self.Porch Block`) (`KismetMathLibrary.MakeTransform` _position (`self.Current Rotation`)))
            (else
              (`InstancedStaticMeshComponent.AddInstance` (`self.Foundattion Block`) (`KismetMathLibrary.MakeTransform` _position (struct)))))))
      (return _balcony_ _position))))

(fn `Init details`
  (params (`Balcony?` :type Boolean) (Floor :type Integer) (Segment :type Integer) (`Segment Width` :type Integer))
  (if (!= Floor 0)
    (if true
      (`self.Calculate random window`
        (:`Finish`
          (if (< (`KismetMathLibrary.RandomInteger` 2) 1)
            (`self.Calculate detail position` (`self.Dryer Length to Face`)
              (:`End`
                (`InstancedStaticMeshComponent.AddInstance` (`self.Dryer`) (`KismetMathLibrary.MakeTransform` (`self.Detail Position`) (`self.Current Rotation`)))))
            (else
              (`self.Calculate detail position` (`self.Air conditionr Length to Face`)
                (:`End`
                  (`InstancedStaticMeshComponent.AddInstance` (`self.AirConditiner`) (`KismetMathLibrary.MakeTransform` (`self.Detail Position`) (`self.Current Rotation`))))))))))))

(fn `UserConstructionScript`
  (bind (_min _max) (`StaticMeshComponent.GetLocalBounds` (`self.Block`)))
  (set `self.Block Bound Radius` (.x _max))
  (set `self.Block Height` (+ (.z _max) 1.0))
  (for _index (range (+ (`self.Floors`) 1))
    (for _index_2 (range (+ (`self.Segments`) 1))
      (for _index_3 (range (+ (`self.Segmetns Width`) 1))
        (if (`self.Check if the block should be put` _index_3 _index_2 _index)
          (bind (_balcony_ _position) (`self.Init Block` _index _index_2 _index_3))
          (set `self.Current Position` _position)
          (`self.Init details` _balcony_ _index _index_2 _index_3))))))