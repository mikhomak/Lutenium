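; Player plane pawn with physics-driven PlaneMovement, machine gun/missile switching and a support attack.
; Tick scales spring-arm length and thrust VFX from input, while acceleration triggers an FOV kick and events toggle trail and wing snow effects.
; A rear safe zone halves incoming power projectiles' max speed and alerts the back-camera widget granted by the BackMirrors upgrade.
; Several debug and experimental paths are empty or disconnected.
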(event `self.ReceiveTick`
  (params (DeltaSeconds :type "Float (single-precision)"))
  (`self.Manage Thrust VFX`)
  (`self.Caclulate Camera Arm Length`)
  (`self.All Power projectiles exit safezone`))

(event `Key|B`
  (params (Key :type "Key Structure"))
  (:`Pressed`
    (`self.SwitchWeapons` (select `bool` (`|EnumEquality` (`self.CurrentWeapon`) "Missile") :`false` "Missile" :`true` "MachineGun" :!type "EPlayerWeapon Enum"))))

(event `self.DotHasChange`
  (params (Dot :type "Float (single-precision)"))
  (`self.Toggle Spawn Rate of Trails VFX` Dot))

(event `self.ReceiveBeginPlay`
  (`/Game/RetroGraphics/Blueprints/FL_RetroGraphics.SetScreenPercentage` 50.0)
  (`self.Toggle Spawn Rate of Trails VFX` 0.0)
  (`self.Create Widgets`)
  (`self.Deactivate both snow VFX`))

(event `self.OnKickInAccelerationEvent`
  (bind _camera (`self.Camera`))
  ;[0 1 0.9134] take off acceleration camera wrap effect
  (bind (_direction _camera_wrap_start_effect) (`Timeline|Camera Wrap Start Effect` :!via `PlayFromStart`)
    (:`Update`
      (`CameraComponent.SetFieldOfView` _camera (`KismetMathLibrary.Lerp` 120.0 125.0 _camera_wrap_start_effect)))
    (:`Finished`
      (bind (_direction_2 _camera_wrap_end_effect) (`Timeline|Camera Wrap End Effect` :!via `PlayFromStart`)
        (:`Update`
          (`CameraComponent.SetFieldOfView` _camera (`KismetMathLibrary.Lerp` 120.0 125.0 _camera_wrap_end_effect)))))))

(event `self.AquieredUpgrade`
  (params (Upgrade :type "EPlayerUpgrade Enum" :default "IncreasedAimRadius"))
  (`self.Aquiere Back Windows Upgrade` Upgrade))

(event `Key|SpaceBar`
  (params (Key :type "Key Structure")))

(event `self.MissileBackSafeZone.OnComponentBeginOverlap`
  (params (OverlappedComponent :type "PrimitiveComponent Object Reference") (OtherActor :type "Actor Object Reference") (OtherComp :type "PrimitiveComponent Object Reference") (OtherBodyIndex :type Integer) (bFromSweep :type Boolean) (SweepResult :type "HitResult Structure (by ref)"))
  (bind _widget_back_camera (`self.Widget Back Camera`))
  (`self.Power Projectiles Enter SafeZone` OtherActor)
  (`/Engine/EditorBlueprintResources/StandardMacros.IsValid` _widget_back_camera
    (:`Is Valid`
      (`/Game/Blueprints/Player/UI/WBP_BackCamera.ProjectileHasEnteredSafeZone` _widget_back_camera))))

(event `self.MissileBackSafeZone.OnComponentEndOverlap`
  (params (OverlappedComponent :type "PrimitiveComponent Object Reference") (OtherActor :type "Actor Object Reference") (OtherComp :type "PrimitiveComponent Object Reference") (OtherBodyIndex :type Integer))
  (bind _widget_back_camera (`self.Widget Back Camera`))
  (`self.Power Projectile Exit SafeZone` OtherActor)
  (`/Engine/EditorBlueprintResources/StandardMacros.IsValid` _widget_back_camera
    (:`Is Valid`
      (`/Game/Blueprints/Player/UI/WBP_BackCamera.ProjectileHasExitSafeZone` _widget_back_camera))))

(event `self.SnowTouchRightWing.OnComponentBeginOverlap`
  (params (OverlappedComponent :type "PrimitiveComponent Object Reference") (OtherActor :type "Actor Object Reference") (OtherComp :type "PrimitiveComponent Object Reference") (OtherBodyIndex :type Integer) (bFromSweep :type Boolean) (SweepResult :type "HitResult Structure (by ref)"))
  ;[0.2292 0.2292 0.2292] Snow VFX
  (`self.Toggle Spawn Rate of Snow VFX` true true :!label _label))

(event `self.SnowTouchRightWing.OnComponentHit`
  (params (HitComponent :type "PrimitiveComponent Object Reference") (OtherActor :type "Actor Object Reference") (OtherComp :type "PrimitiveComponent Object Reference") (NormalImpulse :type "Vector Structure") (Hit :type "HitResult Structure (by ref)"))
  (goto _label))

(event `self.SnowTouchLeftWing.OnComponentBeginOverlap`
  (params (OverlappedComponent :type "PrimitiveComponent Object Reference") (OtherActor :type "Actor Object Reference") (OtherComp :type "PrimitiveComponent Object Reference") (OtherBodyIndex :type Integer) (bFromSweep :type Boolean) (SweepResult :type "HitResult Structure (by ref)"))
  ;[0.2292 0.2292 0.2292] Snow VFX
  (`self.Toggle Spawn Rate of Snow VFX` false true))

(event `Key|Q`
  (params (Key :type "Key Structure"))
  (:`Pressed`
    (`self.BaseSupportAttack`)))

(event `self.OnBaseSupportAttackEvent`
  (params (Target :type "SceneComponent Object Reference"))
  (`KismetSystemLibrary.PrintString` (`KismetStringLibrary.Concat_StrStr` "Ayooooooo" (`KismetSystemLibrary.GetDisplayName` Target))))

(event `self.SnowTouchRightWing.OnComponentEndOverlap`
  (params (OverlappedComponent :type "PrimitiveComponent Object Reference") (OtherActor :type "Actor Object Reference") (OtherComp :type "PrimitiveComponent Object Reference") (OtherBodyIndex :type Integer))
  ;[0.2292 0.2292 0.2292] Snow VFX
  (`self.Toggle Spawn Rate of Snow VFX` true))

(event `self.SnowTouchLeftWing.OnComponentEndOverlap`
  (params (OverlappedComponent :type "PrimitiveComponent Object Reference") (OtherActor :type "Actor Object Reference") (OtherComp :type "PrimitiveComponent Object Reference") (OtherBodyIndex :type Integer))
  ;[0.2292 0.2292 0.2292] Snow VFX
  (`self.Toggle Spawn Rate of Snow VFX` false))

(fn `All Power projectiles exit safezone`)

(fn `Aquiere Back Windows Upgrade`
  (params (Upgrade :type "EPlayerUpgrade Enum" :default "IncreasedAimRadius"))
  (if (`|EnumEquality` Upgrade "BackMirrors")
    (bind _returnvalue (`|CreateWidget` "/Game/Blueprints/Player/UI/WBP_BackCamera.WBP_BackCamera_C"))
    (bind _output_get (set `self.Widget Back Camera` _returnvalue))
    (`UserWidget.AddToViewport` _output_get 0)))

(fn `Caclulate Camera Arm Length`
  (bind _springarm (`self.SpringArm`))
  (if (not (`self.Dash Camera Length?`))
    (bind _output_get (set `self.Current Camera Pitch Backward Length` (`KismetMathLibrary.Lerp` (`KismetMathLibrary.MapRangeClamped` (`KismetMathLibrary.Abs` (`PlaneMovementComponent.Dot` (`self.PlaneMovement`))) 0.0 1.0 0.0 50.0) (`self.Current Camera Pitch Backward Length`) 0.6)))
    (set `SpringArmComponent.TargetArmLength` (- (`KismetMathLibrary.Lerp` (`KismetMathLibrary.MapRangeClamped` (`self.GetThrustInput`) 0.0 1.0 1400.0 1624.0) (`SpringArmComponent.TargetArmLength` _springarm) 0.91) _output_get) _springarm)))

(fn `Create Widgets`
  (bind _returnvalue (`|CreateWidget` "/Game/Blueprints/Player/UI/WBP_HUD.WBP_HUD_C"))
  (bind _output_get (set `self.Widget Altitude` _returnvalue))
  (`UserWidget.AddToViewport` _output_get 0))

(fn `Deactivate both snow VFX`
  (`self.Toggle Spawn Rate of Snow VFX` true)
  (`self.Toggle Spawn Rate of Snow VFX` false))

(fn `EMp debug`
  (bind _empmovementeffect (`PlaneMovementComponent.EmpMovementEffect` (`self.PlaneMovement`)))
  (if (`MovementEffect.Active` _empmovementeffect)
    (`PrimitiveComponent.AddTorqueInRadians` (`self.PlaneBox`) (`KismetMathLibrary.VLerp` (0.0 0.0 0.0) (* (`EmpMovementEffect.RotationDirection` _empmovementeffect) (`EmpMovementEffect.RotationForce` _empmovementeffect)) 0.1) "None" true)))

(fn `Kick in Acceleration Camera Shake`
  (if (`self.Can Camera Shake?`)
    _))

(fn `Manage Thrust VFX`
  (bind _returnvalue (`self.Create Rotator Fro Thrust VFX`))
  (bind _returnvalue_2 (`KismetMathLibrary.Lerp` (`self.GetThrustInput`) (`self.Current thrust value VFX`) 0.8))
  (bind _returnvalue_3 (select `bool` (`KismetMathLibrary.NearlyEqual_FloatFloat` _returnvalue_2) :`false` (`KismetMathLibrary.MapRangeUnclamped` _returnvalue_2 -1.0 1.0 0.0 -500.0) :`true` -80.0))
  ;[1 1 1] Thrust VFX rotation
  (`SceneComponent.K2_SetRelativeRotation` (`self.Left Thurst`) _returnvalue false false)
  (`SceneComponent.K2_SetRelativeRotation` (`self.Right Thrust`) _returnvalue false false)
  (set `self.Thrust rotator` _returnvalue)
  ;[1 1 1] Thrust VFX Length
  (`FXSystemComponent.SetVectorParameter` (`self.Left Thurst`) "User.attractionForce" (`KismetMathLibrary.MakeVector` _returnvalue_3))
  (`FXSystemComponent.SetVectorParameter` (`self.Right Thrust`) "User.attractionForce" (`KismetMathLibrary.MakeVector` _returnvalue_3))
  (set `self.Current thrust value VFX` (`self.GetThrustInput`)))

(fn `Power Projectile Exit SafeZone`
  (params (Object :type "Object Object Reference"))
  (bind _asbp_power_projectile (cast `/Game/Blueprints/Monster/Weapons/BP_PowerProjectile` Object))
  (`/Engine/EditorBlueprintResources/StandardMacros.IsValid` _asbp_power_projectile
    (:`Is Valid`
      (set `ProjectileMovementComponent.MaxSpeed` (`self.MonsterProjectileMaxSpeed`) (`PowerProjectile.ProjectileMovement` _asbp_power_projectile))
      (set `self.Amount Of Projectiles in safe zone` (- (`self.Amount Of Projectiles in safe zone`) 1)))))

(fn `Power Projectiles Enter SafeZone`
  (params (Actor :type "Object Object Reference"))
  (bind _asbp_power_projectile (cast `/Game/Blueprints/Monster/Weapons/BP_PowerProjectile` Actor))
  (`/Engine/EditorBlueprintResources/StandardMacros.IsValid` _asbp_power_projectile
    (:`Is Valid`
      (bind _projectilemovement (`PowerProjectile.ProjectileMovement` _asbp_power_projectile))
      (bind _maxspeed (`ProjectileMovementComponent.MaxSpeed` _projectilemovement))
      (set `self.MonsterProjectileMaxSpeed` _maxspeed)
      (set `ProjectileMovementComponent.MaxSpeed` (/ _maxspeed 2.0) _projectilemovement)
      (set `self.Amount Of Projectiles in safe zone` (+ (`self.Amount Of Projectiles in safe zone`) 1))
      (set `self.bIsAnyProjectilesInSafezone` true))))

(fn `Rotate`
  (params (Yes :type "Float (double-precision)"))
  (set `self.Target Pitch` Yes)
  (if (!= Yes 0.0)
    (`PrimitiveComponent.AddTorqueInRadians` (`self.PlaneBox`) (`KismetMathLibrary.GreaterGreater_VectorRotator` (`KismetMathLibrary.MakeVector` 0.0 (* Yes 5.0)) (`self.K2_GetActorRotation`)) "None" true)))

(fn `Toggle Spawn Rate of Snow VFX`
  (params (`Left or Right?` :type Boolean) (`Activate ?` :type Boolean))
  (`NiagaraComponent.SetVariableFloat` (select `bool` `Left or Right?` :`false` (`self.NS_Snow_Wings_Touch`) :`true` (`self.NS_Snow_Wings_Touch1`)) "User.SpawnRate" (`KismetMathLibrary.SelectFloat` 500.0 0.0 `Activate ?`)))

(fn `Toggle Spawn Rate of Trails VFX`
  (params (Dot :type "Float (double-precision)"))
  (bind _next_trail_spawn_rate (`self.Next Trail Spawn Rate`))
  (`NiagaraComponent.SetVariableFloat` (`self.TrailLeft`) "User.SpawnRate" _next_trail_spawn_rate)
  (`NiagaraComponent.SetVariableFloat` (`self.TrailRight`) "User.SpawnRate" _next_trail_spawn_rate)
  (if (> (`self.Next Trail Spawn Rate`) 0.0)
    (set `self.Next Trail Spawn Rate` 0.0)
    (else
      (set `self.Next Trail Spawn Rate` 200.0))))

(fn `UserConstructionScript`
  (bind _planemovement (`self.PlaneMovement`))
  (set `PlayerPlaneMovementComponent.PlayerPawn` self _planemovement)
  (set `PlaneMovementComponent.PhysicsComponent` (`self.PlaneBox`) _planemovement)
  (set `PlaneMovementComponent.OwnerPawn` self _planemovement))