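; Player plane pawn that hands its flight behavior to a PlaneMovement component.
; The construction script passes the pawn and PlaneMesh to that component and sets tick groups for the mesh and both trails, with the left trail in PrePhysics and the others in PostUpdateWork.
; The event graph is mostly inert: an empty Tick, a zero-impulse Stop input, and disconnected debug draws of velocity and its alignment with the mesh up vector.
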(event `self.ReceiveTick`
  (params (DeltaSeconds :type "Float (single-precision)")))

(event `InputAction|Stop`
  (params (Key :type "Key Structure"))
  (:`Pressed`
    (`PrimitiveComponent.AddImpulse` (`self.PlaneMesh`) (0.0 0.0 0.0) "None" false)))

(fn `UserConstructionScript`
  (bind _planemovement (`self.PlaneMovement`))
  ;[1 1 1] Plane movement setup
  (`PlaneMovementComponent.SetPawn` _planemovement self)
  (`PlaneMovementComponent.SetMesh` _planemovement (`self.PlaneMesh`))
  ;[1 1 1] Tick Group
  (`ActorComponent.SetTickGroup` (`self.Trail right`) "TG_PostUpdateWork")
  (`ActorComponent.SetTickGroup` (`self.Trail left`) "TG_PrePhysics")
  (`ActorComponent.SetTickGroup` (`self.PlaneMesh`) "TG_PostUpdateWork"))